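; BP_StartFinish is an actor that visually marks a start, a finish, both or neither, as set by its Start and Finish flags.
; The construction script maps each flag combination to a ColorSelector value and sets it as a scalar material parameter on three cube components.
; The event graph holds only disabled stub events, so the Blueprint adds no runtime logic.
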(event EventBeginPlay)

(event Collision|EventActorBeginOverlap
  (params (OtherActor :type Actor%20Object%20Reference)))

(event EventTick
  (params (DeltaSeconds :type Float%20%28single-precision%29)))

(fn ConstructionScript
  (if (Variables|Default|GetbFinish)
    (if (Variables|Default|GetbStart)
      (Variables|Default|SetColorSelectorValue 2.0)
      (else
        (Variables|Default|SetColorSelectorValue 1.0)))
    (elif (Variables|Default|GetbStart)
      (Variables|Default|SetColorSelectorValue 0.0)
      (else
        (Variables|Default|SetColorSelectorValue -1.0))))
  (Rendering|Material|SetScalarParameterValueonMaterials (Variables|Default|GetCube1) "ColorSelector" (Variables|Default|GetColorSelectorValue)))